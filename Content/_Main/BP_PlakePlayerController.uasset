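; Player controller that creates the player's HUD widget and fills it with health and mana on possession.
; Possess spawns WBP_PlayerUI, casts the pawn to PlakeCharacter and passes its PlayerStats component to UpdateUI.
; UpdateUI pushes current values and percentages to the widget once, with no recurring refresh in this graph.
; A debug print shows the pawn name; the invalid-stats branch only delays, without retrying.
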(event Custom|CreateUI
  (params (OwningPlayer :type Player%20Controller%20Object%20Reference))
  (bind _returnvalue (UserInterface|CreateWidget "/Game/_Main/UI/WBP_PlayerUI.WBP_PlayerUI_C" OwningPlayer))
  (UserInterface|Viewport|AddtoViewport _returnvalue 0)
  (Variables|Default|SetPlayerUI _returnvalue))

(event EventUpdateUI
  (params (PlayerStats :type Player%20Stats%20Component%20Object%20Reference))
  (Utilities|FlowControl|Sequence
    (:then_0
      (bind _returnvalue (Class|PlayerStatsComponent|GetCurrentHealth PlayerStats)))
    (:then_1
      (bind _returnvalue_2 (Class|PlayerStatsComponent|GetCurrentHealthPercent PlayerStats)))
    (:then_2
      (bind _returnvalue_3 (Class|PlayerStatsComponent|GetCurrentMana PlayerStats)))
    (:then_3
      (bind _returnvalue_4 (Class|PlayerStatsComponent|GetCurrentManaPercent PlayerStats)))
    (:then_4
      (Default|UpdateHealthandMana (Variables|Default|GetPlayerUI) (Math|Float|Truncate _returnvalue) (Math|Float|Truncate _returnvalue_3) _returnvalue_2 _returnvalue_4))))

(event EventTick
  (params (DeltaSeconds :type Float%20%28single-precision%29)))

(event EventPossess
  (params (PossessedPawn :type Pawn%20Object%20Reference))
  (CallFunction|CreateUI self)
  (bind _asplake_character (Utilities|Casting|CastToPlakeCharacter PossessedPawn))
  (bind _returnvalue (Class|PlakeCharacter|GetPlayerStatsComponent _asplake_character))
  (Utilities|IsValid 0
    (:Is%20Valid
      (Class|PlakePlayerController|UpdateUI _returnvalue)
      (Development|PrintString (Utilities|GetDisplayName _asplake_character)))
    (:Is%20Not%20Valid
      (Utilities|FlowControl|Delay 1.0))))

(fn ConstructionScript)